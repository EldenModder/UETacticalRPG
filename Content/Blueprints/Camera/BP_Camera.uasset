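; BP_Camera is the player camera for a tactical RPG, with movement, yaw rotation, boom-arm zoom and unit picking.
; BeginPlay adds the TRPG Enhanced Input context, creates the unit selector widget and caches the level's UnitSpawner.
; Input actions drive movement, rotation and spring-arm length.
; A left-click debug key traces Pawns under the cursor and stores the hit BP_Unit, only while the spawner's CanSpawnUnit is invalid.
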(event Input|EnhancedActionEvents|EnhancedInputActionIA_Scroll
  (params (ActionValue :type Float%20%28double-precision%29) (ElapsedSeconds :type Float%20%28double-precision%29) (TriggeredSeconds :type Float%20%28double-precision%29) (InputAction :type Input%20Action%20Object%20Reference :default "/Game/Inputs/input/IA_Scroll.IA_Scroll"))
  (CallFunction|SetTargetArmLenght (+ (CallFunction|GetTargetArmLenght) (* ActionValue (Variables|Default|GetZoomSpeed)))))

(event Input|EnhancedActionEvents|EnhancedInputActionIA_Move
  (params (ActionValue :type Vector%202D%20Structure) (ElapsedSeconds :type Float%20%28double-precision%29) (TriggeredSeconds :type Float%20%28double-precision%29) (InputAction :type Input%20Action%20Object%20Reference :default "/Game/Inputs/input/IA_Move.IA_Move"))
  (Pawn|Input|AddMovementInput (Transformation|GetActorForwardVector) (.x ActionValue) false)
  (Pawn|Input|AddMovementInput (Transformation|GetActorRightVector) (.y ActionValue) false))

(event Input|EnhancedActionEvents|EnhancedInputActionIA_Rotate
  (params (ActionValue :type Vector%202D%20Structure) (ElapsedSeconds :type Float%20%28double-precision%29) (TriggeredSeconds :type Float%20%28double-precision%29) (InputAction :type Input%20Action%20Object%20Reference :default "/Game/Inputs/input/IA_Rotate.IA_Rotate"))
  (Transformation|AddActorLocalRotation (Math|Rotator|MakeRotator 0.0 0.0 (* (* (.x ActionValue) (Variables|Default|GetRotationSpeed)) (Utilities|Time|GetWorldDeltaSeconds))) false false))

(event EventBeginPlay
  (Input|AddMappingContext (PlayerController|LocalPlayerSubsystems|GetEnhancedInputLocalPlayerSubsystem (Game|GetPlayerController 0)) "/Game/Inputs/IMC_TRPG.IMC_TRPG" 0 "(bIgnoreAllPressedKeysUntilRelease=True,bForceImmediately=False,bNotifyUserSettings=False)")
  (bind _returnvalue (UserInterface|CreateWidget "/Game/Blueprints/Widgets/WBP_UnitSelecter.WBP_UnitSelecter_C"))
  (UserInterface|Viewport|AddtoViewport _returnvalue 0)
  (bind _returnvalue_2 (Actor|GetActorOfClass "/Script/TacticalRPG.UnitSpawner"))
  (Variables|Default|SetUnitSpawner _returnvalue_2))

(event Input|MouseEvents|DebugKeyLeftMouseButton
  (params (Key :type Key%20Structure :default "None") (ActionValue :type Input%20Action%20Value%20Structure))
  (:Pressed
    (bind _unitspawner (Variables|Default|GetUnitSpawner)
      (:then
        (Variables|/Script/TacticalRPG.UnitSpawner|GetbCanSpawnUnit _unitspawner
          (:then)
          (:else
            (bind _actorhitedclass (CallFunction|GetUnitUnderCursor))
            (bind _asbp_unit (Utilities|Casting|CastToBP_Unit _actorhitedclass)
              (:then
                (Variables|Default|SetBP%20Unit _asbp_unit))
              (:CastFailed
                (CallFunction|LogWarning "Not a Unit Actor"))))))
      (:else
        (CallFunction|LogWarning "No UnitSpawner Found")))))

(fn ConstructionScript)

(fn GetTargetArmLenght
  (return (Variables|/Script/Engine.SpringArmComponent|GetTargetArmLength (Variables|Default|GetCameraBoom))))

(fn SetTargetArmLenght
  (params (Target%20Arm%20Length :type Float%20%28single-precision%29))
  (Variables|/Script/Engine.SpringArmComponent|SetTargetArmLength (Variables|Default|GetCameraBoom) Target%20Arm%20Length))

(fn GetUnitUnderCursor
  (return (.HitActor (Collision|BreakHitResult (.HitResult (Class|PlayerController|GetHitResultUnderCursorforObjects (Game|GetPlayerController 0) (Utilities|Array|MakeArray "ObjectTypeQuery3") true))))))